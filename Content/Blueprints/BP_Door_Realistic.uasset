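; BP_Door_Realistic is a door actor that rotates its Door component when its Open and Close events are called.
; Open plays a timeline and Close reverses it.
; Each timeline update adds a scaled Rotation track value to the door's yaw as a relative delta, so motion accumulates per tick instead of setting an absolute angle.
; A disconnected sliding-location variant and a delay remain unused.
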(event `self.Open`
  (bind (_direction _track _rotation) (`Timeline|Timeline` :!label _label)
    (:`Update`
      (`SceneComponent.K2_AddRelativeRotation` (`self.Door`) (`KismetMathLibrary.MakeRotator` 0.0 0.0 (/ _rotation 100.0)) false false))))

(event `self.Close`
  (goto _label :!via `Reverse`))

(fn `UserConstructionScript`
  (`parent.UserConstructionScript`))