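; BP_Door is an interactable door that slides open and closed.
; OnInterect switches on interaction type: Pickup and Enable open it, Disable closes it, and Toggle alternates between both through a FlipFlop.
; Open plays TL_OpenDoor, whose track sets the Door component's relative Y location, and Close reverses that timeline.
; A rotation-based variant remains in the graph but never runs.
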(event `/Game/Blueprints/BPI_Interactable.OnInterect`
  (params (InteractingActor :type "Actor Object Reference (by ref)") (InteractionType :type "/Game/Blueprints/InteractionType_ENUM Enum" :default "NewEnumerator0"))
  (switch `/Game/Blueprints/InteractionType_ENUM` InteractionType
    (:`NewEnumerator0`
      (`self.Open` :!label _label))
    (:`NewEnumerator1`
      (`/Engine/EditorBlueprintResources/StandardMacros.FlipFlop`
        (:`A`
          (goto _label))
        (:`B`
          (`self.Close` :!label _label_2))))
    (:`NewEnumerator2`
      (goto _label))
    (:`NewEnumerator3`
      (goto _label_2))))

(event `Open`
  (bind (_direction _track _rotation) (`Timeline|TL_OpenDoor` :!label _label_3)
    (:`Update`
      (`SceneComponent.K2_SetRelativeLocation` (`self.Door`) (`KismetMathLibrary.MakeVector` 0.0 (* _track -1.5)) false false))))

(event `Close`
  (goto _label_3 :!via `Reverse`))

(fn `UserConstructionScript`)