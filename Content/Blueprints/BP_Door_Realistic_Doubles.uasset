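; Double door Blueprint that swings two door components, Door and Door2, through Open and Close events.
; Open plays a Timeline and Close reverses it.
; Each Timeline update adds a relative yaw delta to both doors from the Rotation track divided by a constant, so motion accumulates per update rather than setting an absolute angle.
; Nothing in this graph calls Open or Close, apart from an unconnected delay chain.
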(event `self.ReceiveBeginPlay`
  (`parent.ReceiveBeginPlay`))

(event `self.Open`
  (bind (_direction _track _rotation) (`Timeline|Timeline` :!label _label)
    (:`Update`
      (bind _returnvalue (/ _rotation 60.0))
      (bind _result (`/Engine/EditorBlueprintResources/StandardMacros.NegateFloat` _returnvalue)
        (:`  `
          (`SceneComponent.K2_AddRelativeRotation` (`self.Door`) (`KismetMathLibrary.MakeRotator` 0.0 0.0 _result) false false)
          (`SceneComponent.K2_AddRelativeRotation` (`self.Door2`) (`KismetMathLibrary.MakeRotator` 0.0 0.0 _returnvalue) false false))))))

(event `self.Close`
  (goto _label :!via `Reverse`))

(fn `UserConstructionScript`
  (`parent.UserConstructionScript`))