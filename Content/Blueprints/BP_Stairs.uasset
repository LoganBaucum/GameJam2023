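; BP_Stairs is a stairs actor that changes its height when triggered by Open and Close events.
; Open plays a Timeline and Close reverses it, with each update setting the root component's world Z scale from the ScaleOverTime track while X and Y stay at one.
; Scaling the root stretches or shrinks the whole actor vertically.
; A disconnected Door2 scaling node and an unused Door reference remain in the graph.
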(event `self.Open`
  (bind (_direction _scaleovertime) (`Timeline|Timeline` :!label _label)
    (:`Update`
      (`SceneComponent.SetWorldScale3D` (`self.DefaultSceneRoot`) (`KismetMathLibrary.MakeVector` 1.0 1.0 _scaleovertime)))))

(event `self.Close`
  (goto _label :!via `Reverse`))

(fn `UserConstructionScript`
  (`parent.UserConstructionScript`))